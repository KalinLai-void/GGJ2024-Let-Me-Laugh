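; BP_Interactable is a gift pickup that the first-person player takes into their hand.
; Tick rolls a random MeshInfo once while the player holds nothing, playing a tip cue for positively liked items.
; Interact passes that info and a random like increase to the character, then respawns its class on GiftPoint without collision and destroys itself.
; The character's IsTaking flag keeps the held copy from rerolling.
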(event Custom|GetMesh
  (Variables|Default|SetMesh%20Info (CallFunction|RandomMesh))
  (Variables|Default|SetisGenerated true))

(event EventTick
  (params (DeltaSeconds :type Float%20%28single-precision%29))
  (bind _audiocomp (Variables|Default|GetAudioComp))
  (bind _asbp_first_person_character (Utilities|Casting|CastToBP_FirstPersonCharacter (Game|Player|GetPlayerPawn 0)))
  (if (and (not (Variables|/Game/FirstPerson/Blueprints/BP_FirstPersonCharacter.BP_FirstPersonCharacter_C|GetisTaking _asbp_first_person_character)) (not (Variables|Default|GetisGenerated)))
    (CallFunction|GetMesh)
    (if (.isLikePositive (Utilities|Struct|BreakS_MeshInfo (Variables|Default|GetMesh%20Info)))
      (Audio|Components|Audio|SetSound _audiocomp "/Game/_GGJ2024/Audio/Tip_Cue.Tip_Cue")
      (Audio|Components|Audio|Play _audiocomp 0.0)
      (else
        (Audio|Components|Audio|SetSound _audiocomp 0)))))

(event EventInteract
  (bind _mesh_info (Variables|Default|GetMesh%20Info))
  (bind (_likevalue_min _likevalue_max _actor) (Utilities|Struct|BreakS_MeshInfo _mesh_info))
  (bind _asbp_first_person_character (Utilities|Casting|CastToBP_FirstPersonCharacter (Game|Player|GetPlayerPawn 0)))
  (Variables|/Game/FirstPerson/Blueprints/BP_FirstPersonCharacter.BP_FirstPersonCharacter_C|SetisTaking _asbp_first_person_character true)
  (Variables|/Game/FirstPerson/Blueprints/BP_FirstPersonCharacter.BP_FirstPersonCharacter_C|SetMeshInfo _asbp_first_person_character _mesh_info)
  (Variables|/Game/FirstPerson/Blueprints/BP_FirstPersonCharacter.BP_FirstPersonCharacter_C|SetLikeIncrease _asbp_first_person_character (Math|Random|RandomFloatinRange _likevalue_min _likevalue_max))
  (ChildActorComponent|SetChildActorClass (Variables|/Game/FirstPerson/Blueprints/BP_FirstPersonCharacter.BP_FirstPersonCharacter_C|GetGiftPoint _asbp_first_person_character) (Utilities|GetClass self))
  (Collision|SetActorEnableCollision (Variables|/Script/Engine.ChildActorComponent|GetChildActor (Variables|/Game/FirstPerson/Blueprints/BP_FirstPersonCharacter.BP_FirstPersonCharacter_C|GetGiftPoint _asbp_first_person_character)) false)
  (bind _asbp_interactable (Utilities|Casting|CastToBP_Interactable (Variables|/Script/Engine.ChildActorComponent|GetChildActor (Variables|/Game/FirstPerson/Blueprints/BP_FirstPersonCharacter.BP_FirstPersonCharacter_C|GetGiftPoint _asbp_first_person_character))))
  (Transformation|SetRelativeTransform (Variables|/Game/FirstPerson/Blueprints/BP_FirstPersonCharacter.BP_FirstPersonCharacter_C|GetGiftPoint _asbp_first_person_character) (Variables|/Game/FirstPerson/Blueprints/BP_FirstPersonCharacter.BP_FirstPersonCharacter_C|GetOriginTransform _asbp_first_person_character) false false)
  (Audio|Components|Audio|Stop (Variables|BP_Interactable_C|GetAudioComp _asbp_interactable))
  (Actor|DestroyActor))

(fn ConstructionScript)