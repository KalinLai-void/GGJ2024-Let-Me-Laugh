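; BP_Door is an interactable door that alternates between opening and closing each time Interact is called.
; A FlipFlop plays or reverses a timeline whose track sets the static mesh's relative yaw.
; Opening starts the open sound immediately and stops the close sound, while closing waits briefly before playing the close sound and stopping the open one.
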(event EventInteract
  (Utilities|FlowControl|FlipFlop
    (:A
      (Audio|Components|Audio|Stop (Variables|Default|GetCloseDoor))
      (Audio|Components|Audio|Play (Variables|Default|GetOpenDoor) 0.0)
      (bind _newtrack_0 (Timeline|Timeline Play)
        (:Update
          (Transformation|SetRelativeRotation (Variables|Default|GetStaticMesh) (Math|Rotator|MakeRotator 0.0 0.0 _newtrack_0) false false))))
    (:B
      (Utilities|FlowControl|Sequence
        (:then_0
          (Timeline|Timeline Reverse))
        (:then_1
          (Utilities|FlowControl|Delay 0.8)
          (Audio|Components|Audio|Play (Variables|Default|GetCloseDoor) 0.0)
          (Audio|Components|Audio|Stop (Variables|Default|GetOpenDoor)))))))

(fn ConstructionScript)