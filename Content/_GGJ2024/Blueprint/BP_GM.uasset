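; BP_GM runs the level's countdown and triggers the lose screen when time runs out.
; On BeginPlay it starts a looping one-second timer that calls the Timer function.
; Each call decrements TimerValue and converts it to text in TimeToText.
; At zero it removes all widgets and adds WB_LoseGame to the viewport, without clearing the looping timer.
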(event EventBeginPlay
  (Utilities|Time|SetTimerbyFunctionName 0 "Timer" 1.0 true))

(fn ConstructionScript)

(fn Timer
  (if (== (Variables|Default|GetTimerValue) 0)
    ;[1 1 1] Loss
    (Viewport|RemoveAllWidgets)
    (bind _returnvalue (UserInterface|CreateWidget "/Game/_GGJ2024/Blueprint/Widget/LoseGame/WB_LoseGame.WB_LoseGame_C"))
    (UserInterface|Viewport|AddtoViewport _returnvalue 0)
    (else
      (bind _output_get (Variables|Default|SetTimerValue (- (Variables|Default|GetTimerValue) 1)))
      (bind _output_get_2 (Variables|Default|SetTimerValue _output_get))
      (Variables|Default|SetTimeToText (Utilities|TimetoText (Math|Conversions|ToFloat(Integer) _output_get_2))))))